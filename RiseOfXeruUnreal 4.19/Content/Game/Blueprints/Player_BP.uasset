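; Player Blueprint that starts the background music and manages the main menu and game menu widgets.
; On BeginPlay it plays the music cue, creates the main menu and sets UI-only input focused on it.
; PlayButtonHit creates the game menu, passes it a reference to the main menu and moves focus to it.
; ExitButtonHit removes the game menu from the viewport.
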(event Custom|PlayButtonHit
  ;[1 1 1] Create the game menu widget when the play button is pressed and the right number of roles is selected
  (bind _returnvalue (UserInterface|CreateWidget "/Game/Game/Blueprints/GameMenu.GameMenu_C"))
  (Variables|/Game/Game/Blueprints/GameMenu.GameMenu_C|SetMainMenu_BP _returnvalue (stale EventBeginPlay _returnvalue))
  (UserInterface|Viewport|AddtoViewport _returnvalue 1)
  (Input|SetInputModeUIOnly (Game|GetPlayerController 0) _returnvalue "DoNotLock"))

(event Custom|ExitButtonHit
  ;[1 1 1] Remove the game menu from the viewport when it is exited
  (Widget|RemovefromParent (stale Custom|PlayButtonHit _returnvalue)))

(event EventBeginPlay
  ;[1 1 1] Create the main menu widget and start the background music playing
  (Audio|PlaySound2D "/Game/Game/Audio/MusicCue.MusicCue" 0.2)
  (bind _returnvalue (UserInterface|CreateWidget "/Game/Game/Blueprints/MainMenu_BP.MainMenu_BP_C"))
  (UserInterface|Viewport|AddtoViewport _returnvalue 0)
  (Input|SetInputModeUIOnly (Game|GetPlayerController 0) _returnvalue "DoNotLock"))

(fn ConstructionScript)